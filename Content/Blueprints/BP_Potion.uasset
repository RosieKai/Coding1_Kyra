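; Potion actor that relocates its Cube component to a random spawn point whenever the cube sits at the world origin.
; Tick checks the Cube's world location against zero, waits through a short Delay, then picks a random BP_PotionSpawnLocation actor and moves the cube slightly above it.
; Only the component is moved, without sweep; BeginPlay and overlap events hold no logic.
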(event EventBeginPlay)

(event Collision|EventActorBeginOverlap
  (params (OtherActor :type Actor%20Object%20Reference)))

(event EventTick
  (params (DeltaSeconds :type Float%20%28single-precision%29))
  (if (Utilities|Operators|EqualEqual :A (Transformation|GetWorldLocation (Variables|Default|GetCube)))
    (Utilities|FlowControl|Delay 1.0)
    (bind _outactors (Actor|GetAllActorsOfClass "/Game/Blueprints/BP_PotionSpawnLocation.BP_PotionSpawnLocation_C"))
    (Transformation|SetWorldLocation (Variables|Default|GetCube) (+ (Transformation|GetActorLocation (.OutItem (Utilities|Array|Random _outactors))) "0.000000,0.000000,50.000000") false false)))

(fn ConstructionScript)