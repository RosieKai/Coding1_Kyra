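; BP_Dave is an actor with a physics Cube, apparently the player, that returns to its starting position.
; BeginPlay stores the Cube's location; Tick moves the actor back there after a short delay when the Cube drops below a height threshold, briefly disabling physics.
; An idle timer, never reset by movement, triggers the same reset without the initial delay about every minute if the Cube is simulating physics.
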(event Custom|CheckIdle
  (bind _cube (Variables|Default|GetCube))
  (if (> (Variables|Default|GetidleTime) 6e+01)
    (if (Physics|IsSimulatingPhysics (Variables|Default|GetCube) "None")
      (Variables|Default|SetidleTime 0.0)
      (Transformation|SetActorLocation (Variables|Default|GetoriginLocation) false false)
      (Physics|SetSimulatePhysics _cube false)
      (Utilities|FlowControl|Delay 0.2)
      (Physics|SetSimulatePhysics _cube true)
      (else
        (Variables|Default|SetidleTime 0.0)))))

(event EventBeginPlay
  (Variables|Default|SetoriginLocation (Transformation|GetWorldLocation (Variables|Default|GetCube))))

(event Collision|EventActorBeginOverlap
  (params (OtherActor :type Actor%20Object%20Reference)))

(event EventTick
  (params (DeltaSeconds :type Float%20%28single-precision%29))
  (bind _cube (Variables|Default|GetCube))
  (Variables|Default|SetidleTime (+ (Variables|Default|GetidleTime) DeltaSeconds))
  (CallFunction|CheckIdle)
  (if (< (.z (Transformation|GetWorldLocation (Variables|Default|GetCube))) -1e+02)
    (Utilities|FlowControl|Delay 0.5)
    (Transformation|SetActorLocation (Variables|Default|GetoriginLocation) false false)
    (Physics|SetSimulatePhysics _cube false)
    (Utilities|FlowControl|Delay 0.2)
    (Physics|SetSimulatePhysics _cube true)))

(fn ConstructionScript)