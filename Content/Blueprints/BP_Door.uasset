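; BP_Door is a locked door that the player character opens with a key on contact.
; A hit on the Cube component checks the third-person character's TotalKeys; with a key, it spends one, destroys the door and prints the remaining count.
; Without a key it prints a refusal message, throttled by the MessAble flag and a short delay so repeated hits do not spam it.
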(event OnComponentHit(Cube)
  (params (HitComponent :type Primitive%20Component%20Object%20Reference) (OtherActor :type Actor%20Object%20Reference) (OtherComp :type Primitive%20Component%20Object%20Reference) (NormalImpulse :type Vector :default "0, 0, 0") (Hit :type Hit%20Result%20Structure%20%28by%20ref%29))
  (bind _asbp_third_person_character (Utilities|Casting|CastToBP_ThirdPersonCharacter OtherActor))
  (if (> (Variables|/Game/ThirdPerson/Blueprints/BP_ThirdPersonCharacter.BP_ThirdPersonCharacter_C|GettotalKeys _asbp_third_person_character) 0) ; if condition is true; else
    (Math|Integer|DecrementInt (Variables|/Game/ThirdPerson/Blueprints/BP_ThirdPersonCharacter.BP_ThirdPersonCharacter_C|GettotalKeys _asbp_third_person_character) ; remove one key
      (:%20%20
        (Actor|DestroyActor) ; kick down door
        (Development|PrintString (Utilities|String|Append "Total Keys: " (Utilities|String|ToString(Integer) (Variables|/Game/ThirdPerson/Blueprints/BP_ThirdPersonCharacter.BP_ThirdPersonCharacter_C|GettotalKeys _asbp_third_person_character))))))
    (elif (Variables|Default|GetmessAble)
      (Development|PrintString "Come back with a warrant")
      (Variables|Default|SetmessAble false)
      (Utilities|FlowControl|Delay 1.0)
      (Variables|Default|SetmessAble true))))

(event EventBeginPlay
  (Variables|Default|SetmessAble true))

(event Collision|EventActorBeginOverlap
  (params (OtherActor :type Actor%20Object%20Reference)))

(event EventTick
  (params (DeltaSeconds :type Float%20%28single-precision%29)))

(fn ConstructionScript)