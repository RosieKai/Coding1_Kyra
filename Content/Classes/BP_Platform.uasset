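; BP_Platform is a moving platform actor that travels between its Start and End components.
; On BeginPlay it hides both endpoint components and plays PlatformTimeline.
; Each timeline update sets the Platform component's world location by linearly interpolating between the two endpoints' world locations using the track value, without sweeping.
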(event Custom|HideStartEnd
  (Rendering|SetVisibility (Variables|Default|Getstart) false false)
  (Rendering|SetVisibility (Variables|Default|Getend) false false))

(event EventBeginPlay
  (CallFunction|HideStartEnd)
  (bind _newtrack_0 (Timeline|Platform%20Timeline Play)
    (:Update
      (Transformation|SetWorldLocation (Variables|Default|GetPlatform) (Math|Vector|Lerp(Vector) (Transformation|GetWorldLocation (Variables|Default|Getstart)) (Transformation|GetWorldLocation (Variables|Default|Getend)) _newtrack_0) false false))))

(fn ConstructionScript)