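; BP_Item is an item actor that rolls its stats by type at BeginPlay and demonstrates an attack on an enemy.
; Its Constructor function sets Damage for weapons, consumables or tools, giving unnamed weapons a shuffled name.
; After printing stats and a delay, it lowers a found BP_Enemy's Health by scaled Damage.
; A Sequence also starts a Timeline that offsets the sphere vertically from its starting position.
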(event EventBeginPlay
  (Utilities|FlowControl|Sequence ; Can run code after code even if one part is broken
    (:then_0
      (CallFunction|Constructor)
      (Development|PrintString (Utilities|String|Append "Name: " (Variables|Default|GetName) ", Damage: " (Utilities|String|ToString(Integer) (Variables|Default|GetDamage))) true true "(R=0.000000,G=0.660000,B=1.000000,A=1.000000)" 5.0)
      (Utilities|FlowControl|Delay 5.0)
      (bind _returnvalue (Actor|GetActorOfClass "/Game/Blueprints/BP_Enemy.BP_Enemy_C"))
      (CallFunction|Attack _returnvalue)
      (Development|PrintString "DIE"))
    (:then_1
      (Variables|Default|SetSphereLocation (Transformation|GetWorldLocation (Variables|Default|GetSphere)))
      (bind _newtrack_0 (Timeline|Timeline Play)
        (:Update
          (Transformation|SetRelativeLocation (Variables|Default|GetSphere) (Math|Vector|MakeVector (.x (Variables|Default|GetSphereLocation)) (.y (Variables|Default|GetSphereLocation)) (+ (.z (Variables|Default|GetSphereLocation)) (Math|Float|Lerp 0.0 1e+02 _newtrack_0))) false false))))))

(event Collision|EventActorBeginOverlap
  (params (OtherActor :type Actor%20Object%20Reference)))

(event EventTick
  (params (DeltaSeconds :type Float%20%28single-precision%29)))

(fn ConstructionScript)

(fn Constructor
  (bind _weaponnames (Variables|Default|GetWeaponNames))
  (switch Utilities|FlowControl|Switch|SwitchonItemType (Variables|Default|GetType)
    (:NewEnumerator0
      (Variables|Default|SetDamage (Math|Random|RandomIntegerinRange 3 7))
      (if (Utilities|Enum|Equal(Enum) (Variables|Default|GetName) "")
        (Utilities|Array|Shuffle _weaponnames)
        (Variables|Default|SetName (Utilities|Array|Get(acopy) _weaponnames))))
    (:NewEnumerator1
      (Variables|Default|SetDamage 0))
    (:NewEnumerator2
      (Variables|Default|SetDamage 1))))

(fn Attack
  (params (GivenEnemy :type BP%20Enemy%20Object%20Reference))
  (Variables|/Game/Blueprints/BP_Enemy.BP_Enemy_C|SetHealth GivenEnemy (- (Variables|/Game/Blueprints/BP_Enemy.BP_Enemy_C|GetHealth GivenEnemy) (* (Math|Conversions|ToFloat(Integer) (Variables|Default|GetDamage)) 0.01))))